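; BP_MenuGameMode is the menu game mode, providing timeline-driven in and out animations for widget buttons.
; Each event stores the passed button as Target, then plays one shared timeline forward from the start or in reverse from the end.
; Timeline updates write the Progress scalar to dynamic materials on the button's Normal, Hovered and Pressed styles, so only the most recently passed button animates.
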(event `EVent_WidgetTimeLine_ButtonIn`
  (params (Widget_Button_in :type "Button Object Reference (by ref)"))
  (bind (_widgetstyle_normal _widgetstyle_hovered _widgetstyle_pressed) (break `ButtonStyle` (`Button.WidgetStyle` (`self.Target`))))
  (set `self.Target` Widget_Button_in)
  (bind (_direction _set_buttonmaterlai_progress) (`Timeline|时间轴` :!via `PlayFromStart` :!label _label)
    (:`Update`
      (`MaterialInstanceDynamic.SetScalarParameterValue` (`WidgetBlueprintLibrary.GetDynamicMaterial` _widgetstyle_normal) "Progress" _set_buttonmaterlai_progress)
      (`MaterialInstanceDynamic.SetScalarParameterValue` (`WidgetBlueprintLibrary.GetDynamicMaterial` _widgetstyle_hovered) "Progress" _set_buttonmaterlai_progress)
      (`MaterialInstanceDynamic.SetScalarParameterValue` (`WidgetBlueprintLibrary.GetDynamicMaterial` _widgetstyle_pressed) "Progress" _set_buttonmaterlai_progress))))

(event `EVent_WidgetTimeLine_ButtonOut`
  (params (Widget_Button_out :type "Button Object Reference (by ref)"))
  (set `self.Target` Widget_Button_out)
  (goto _label :!via `ReverseFromEnd`))

(fn `UserConstructionScript`)