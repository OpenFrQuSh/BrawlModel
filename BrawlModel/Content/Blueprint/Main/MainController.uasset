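; Player controller that feeds Enhanced Input to the player character.
; On BeginPlay it caches the Player character and registers the input mapping context on the local player subsystem.
; Every phase of the AD and WS axis actions passes its value to the character's matching functions, while Space calls the character only when the action completes.
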(event `self.ReceiveBeginPlay`
  (bind _asplayer (cast `/Game/Blueprint/Main/Player` (`GameplayStatics.GetPlayerCharacter` 0)))
  (set `self.玩家` _asplayer)
  (`EnhancedInputSubsystemInterface.AddMappingContext` (subsystem `EnhancedInputLocalPlayerSubsystem`) "/Game/Blueprint/Main/EnhanceInput/InputMappingContext.InputMappingContext" 0 (struct)))

(event `EnhancedInput|/Game/Blueprint/Main/EnhanceInput/AD`
  (params (ActionValue :type "Float (double-precision)") (ElapsedSeconds :type "Float (double-precision)") (TriggeredSeconds :type "Float (double-precision)") (InputAction :type "InputAction Object Reference" :default "/Game/Blueprint/Main/EnhanceInput/AD.AD"))
  (:`Triggered`
    (`/Game/Blueprint/Main/Player.AD` (`self.玩家`) ActionValue :!label _label))
  (:`Started`
    (goto _label))
  (:`Ongoing`
    (goto _label))
  (:`Canceled`
    (goto _label))
  (:`Completed`
    (goto _label)))

(event `EnhancedInput|/Game/Blueprint/Main/EnhanceInput/WS`
  (params (ActionValue :type "Float (double-precision)") (ElapsedSeconds :type "Float (double-precision)") (TriggeredSeconds :type "Float (double-precision)") (InputAction :type "InputAction Object Reference" :default "/Game/Blueprint/Main/EnhanceInput/WS.WS"))
  (:`Triggered`
    (`/Game/Blueprint/Main/Player.WS` (`self.玩家`) ActionValue :!label _label_2))
  (:`Started`
    (goto _label_2))
  (:`Ongoing`
    (goto _label_2))
  (:`Canceled`
    (goto _label_2))
  (:`Completed`
    (goto _label_2)))

(event `EnhancedInput|/Game/Blueprint/Main/EnhanceInput/Space`
  (params (ActionValue :type Boolean) (ElapsedSeconds :type "Float (double-precision)") (TriggeredSeconds :type "Float (double-precision)") (InputAction :type "InputAction Object Reference" :default "/Game/Blueprint/Main/EnhanceInput/Space.Space"))
  (:`Completed`
    (`/Game/Blueprint/Main/Player.Space` (`self.玩家`))))

(fn `UserConstructionScript`)